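; Buildable storage workbench variant, a child Blueprint that leans on its parent class for use and lifecycle behavior.
; BeginPlay, EndPlay, OnUse, build effect template and sampling checks only forward to the parent.
; Highlight, buildable visibility and construction script graphs are empty stubs.
; The storage getters supply no background and report that no custom color is used, with black as the placeholder value.
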(event `self.ReceiveBeginPlay`
  (`parent.ReceiveBeginPlay`))

(event `ShowHighlightEffect`
  (params (ExpectedState :type Integer)))

(event `DestroyHighlightEffect`)

(event `FGUseableInterface.OnUse`
  (params (byCharacter :type "FGCharacterPlayer Object Reference") (state :type "UseState Structure (by ref)"))
  (`parent.OnUse` byCharacter state))

(event `self.UpdateBuildableVisibility`
  (params (isVisible :type Boolean) (isTutorialComplete :type Boolean)))

(event `self.ReceiveEndPlay`
  (params (EndPlayReason :type "EEndPlayReason Enum" :default "Destroyed"))
  (`parent.ReceiveEndPlay` EndPlayReason))

(event `SetHighlightState`
  (params (NewHighlightState :type Integer)))

(fn `CanBeSampled`
  (returns (ReturnValue :type Boolean))
  (bind _returnvalue (`parent.CanBeSampled`))
  (return _returnvalue))

(fn `GetBuildEffectTemplate`
  (returns (ReturnValue :type "FGMaterialEffect_Build Soft Class Reference"))
  (bind _returnvalue (`parent.GetBuildEffectTemplate`))
  (return _returnvalue))

(fn `GetStorageBackground`
  (returns (Background :type "Texture2D Object Reference"))
  (return null))

(fn `GetStorageColor`
  (returns (Color :type "LinearColor Structure") (UsesColor :type Boolean))
  (return (struct) false))

(fn `OnRep_mHighlightEffectState`)

(fn `UserConstructionScript`)